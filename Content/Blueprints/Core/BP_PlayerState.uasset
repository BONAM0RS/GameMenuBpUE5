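; BP_PlayerState holds the player's progression data: name, level, experience, money, current robot type and unlocked robot types.
; On BeginPlay it loads starting values from the "Start" row of DT_PlayerSettings and unlocks the starting robot.
; Setters broadcast change dispatchers for everything but name, and these are unbound on destroy.
; Add and Remove helpers accept only positive amounts, and RemoveMoney never drops the balance below zero.
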(event Custom|Add%20Money
  (params (Value :type Integer))
  (if (> Value 0)
    (CallFunction|SetMoney (+ Value (Variables|Default|GetMoney)))))

(event Custom|Set%20Money
  (params (Value :type Integer))
  (bind _output_get (Variables|Default|SetMoney Value))
  (Default|CallOnMoneyChanged _output_get))

(event Custom|Unlock%20Robot
  (params (Robot%20Type :type E_RobotType%20Enum%20%28by%20ref%29 :default "NewEnumerator0"))
  (Utilities|Array|Add (Variables|Default|GetUnlockedRobotTypes) Robot%20Type)
  (Default|CallOnUnlockedRobot Robot%20Type))

(event Custom|Remove%20Money
  (params (Value :type Integer))
  (bind _money (Variables|Default|GetMoney))
  (bind _returnvalue (- _money Value))
  (if (> Value 0)
    (if (>= _returnvalue 0)
      (CallFunction|SetMoney _returnvalue))))

(event Custom|Set%20Level
  (params (Value :type Integer))
  (bind _output_get (Variables|Default|SetLevel Value))
  (Default|CallOnLevelChanged _output_get))

(event Custom|Set%20Exp
  (params (Value :type Integer))
  (bind _output_get (Variables|Default|SetExp Value))
  (Default|CallOnExpChanged _output_get))

(event Custom|Set%20Robot%20Type
  (params (RobotType :type E_RobotType%20Enum :default "NewEnumerator0"))
  (bind _output_get (Variables|Default|SetRobotType RobotType))
  (Default|CallOnRobotTypeChanged _output_get))

(event Custom|Add%20Level
  (params (Value :type Integer))
  (if (> Value 0)
    (CallFunction|SetLevel (+ Value (Variables|Default|GetLevel)))))

(event Custom|Add%20Exp
  (params (Value :type Integer))
  (if (> Value 0)
    (CallFunction|SetExp (+ Value (Variables|Default|GetExp)))))

(event Custom|Set%20Name
  (params (String :type String))
  (Variables|Default|SetName String))

(event EventBeginPlay
  (bind _returnvalue (Utilities|GetDataTableRow "/Game/DataTables/Settings/DT_PlayerSettings.DT_PlayerSettings" "Start")
    (:then
      (CallFunction|SetName (.Name (Utilities|Struct|BreakS_PlayerSettings _returnvalue)))
      (CallFunction|SetLevel (.Level (Utilities|Struct|BreakS_PlayerSettings _returnvalue)))
      (CallFunction|SetExp (.Exp (Utilities|Struct|BreakS_PlayerSettings _returnvalue)))
      (CallFunction|SetMoney (.Money (Utilities|Struct|BreakS_PlayerSettings _returnvalue)))
      (CallFunction|SetRobotType (.RobotType (Utilities|Struct|BreakS_PlayerSettings _returnvalue)))
      (Variables|Default|SetUnlockedRobotTypes (.UnclockedRobotTypes (Utilities|Struct|BreakS_PlayerSettings _returnvalue)))
      (CallFunction|UnlockRobot (.RobotType (Utilities|Struct|BreakS_PlayerSettings _returnvalue))))))

(event EventDestroyed
  (EventDispatchers|UnbindallEventsfromOnLevelChanged)
  (EventDispatchers|UnbindallEventsfromOnExpChanged)
  (EventDispatchers|UnbindallEventsfromOnMoneyChanged)
  (EventDispatchers|UnbindallEventsfromOnRobotTypeChanged)
  (EventDispatchers|UnbindallEventsfromOnUnlockedRobot))

(fn ConstructionScript)